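; BP_ForceField is a damageable force field actor with four orbiting components.
; On BeginPlay, four RotatingMovement components are each bound to their own Orbit component to drive the spin.
; AnyDamage subtracts from Life and destroys the actor only when Life equals exactly zero, as the clamp node is left unused.
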(event `self.ReceiveBeginPlay`
  (`MovementComponent.SetUpdatedComponent` (`self.RotatingMovement`) (`self.Orbit1`))
  (`MovementComponent.SetUpdatedComponent` (`self.RotatingMovement1`) (`self.Orbit2`))
  (`MovementComponent.SetUpdatedComponent` (`self.RotatingMovement2`) (`self.Orbit3`))
  (`MovementComponent.SetUpdatedComponent` (`self.RotatingMovement3`) (`self.Orbit4`)))

(event `self.ReceiveAnyDamage`
  (params (Damage :type "Float (single-precision)") (DamageType :type "DamageType Object Reference") (InstigatedBy :type "Controller Object Reference") (DamageCauser :type "Actor Object Reference"))
  (bind _output_get (set `self.Life` (- (`self.Life`) Damage)))
  (if (== _output_get 0.0)
    (`self.K2_DestroyActor`)))

(fn `UserConstructionScript`)