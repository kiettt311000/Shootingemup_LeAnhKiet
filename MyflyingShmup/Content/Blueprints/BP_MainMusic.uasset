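; BP_MainMusic is a Blueprint that plays the game's main music through an Audio component.
; On BeginPlay it sets the sound and fades it in over a short time.
; A WHENStart event fades the current track out, waits slightly less than the fade length, then sets the sound again and fades it back in.
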(event `self.ReceiveBeginPlay`
  (`AudioComponent.SetSound` (`self.Audio`) null)
  (`AudioComponent.FadeIn` (`self.Audio`) 2.0 1.0 0.0 "Linear"))

(event `WHENStart`
  (`AudioComponent.FadeOut` (`self.Audio`) 2.0 0.0 "Linear")
  (`KismetSystemLibrary.Delay` 1.5)
  (`AudioComponent.SetSound` (`self.Audio`) null)
  (`AudioComponent.FadeIn` (`self.Audio`) 2.0 1.0 0.0 "Linear"))

(fn `UserConstructionScript`)