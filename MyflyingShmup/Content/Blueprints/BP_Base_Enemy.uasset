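; Base enemy actor that takes damage from overlapping BP_Projectile actors and updates a health bar in its widget component.
; A non-lethal hit plays a sound and briefly flashes all static meshes with a damage overlay material.
; At zero health it plays a sound, has the player controller shake the camera and add MaxHealth as score, spawns EnemyDeath and destroys itself.
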(event `self.ReceiveBeginPlay`
  (set `self.Health` (`self.MaxHealth`)))

(event `self.ReceiveActorBeginOverlap`
  (params (OtherActor :type "Actor Object Reference"))
  (bind _asbp_projectile (cast `/Game/Blueprints/BP_Projectile` OtherActor))
  (`self.ApplyDamage` (`/Game/Blueprints/BP_Projectile.Damage` _asbp_projectile))
  ; Check if Enemy Health is Zero, it death
  (if (<= (`self.Health`) 0.0)
    (`GameplayStatics.PlaySound2D` "/Game/Sci-Fi_Shots_Pack2_Game_Of_Weapons/Wave/THISONE.THISONE" 1.0 1.0 0.0 null null)
    (`|ExecutionSequence`
      (:`then_0`
        (bind _asmy_playercontroller (cast `/Game/Framework/MyPlayercontroller` (`GameplayStatics.GetPlayerController` 0)))
        (`/Game/Framework/MyPlayercontroller.ApplyCameraShake` _asmy_playercontroller)
        (`/Game/Framework/MyPlayercontroller.AddScore` _asmy_playercontroller (`self.MaxHealth`)))
      (:`then_1`
        (`|SpawnActorFromClass` "/Game/Particles/EnemyDeath.EnemyDeath_C" (`KismetMathLibrary.MakeTransform` (`self.K2_GetActorLocation`)) "AlwaysSpawn" "MultiplyWithRoot" null null))
      (:`then_2`
        (`self.K2_DestroyActor`)))
    (else
      (`GameplayStatics.PlaySound2D` "/Game/Sci-Fi_Shots_Pack2_Game_Of_Weapons/Cue/THISONE1.THISONE1" 1.0 1.0 0.0 null null)
      (for _array_element (`self.K2_GetComponentsByClass` "/Script/Engine.StaticMeshComponent")
        (`MeshComponent.SetOverlayMaterial` _array_element "/Game/Material/MI_DamageFlash.MI_DamageFlash"))
      (`KismetSystemLibrary.Delay` 0.2)
      (for _array_element_2 (`self.K2_GetComponentsByClass` "/Script/Engine.StaticMeshComponent")
        (`MeshComponent.SetOverlayMaterial` _array_element_2 null)))))

(event `ApplyDamage`
  (params (Damage :type "Float (double-precision)"))
  ; Set progress bar widget within widget component
  (set `self.Health` (- (`self.Health`) Damage))
  (bind _aswbp_enemy_health_bar (cast `/Game/UI/WBP_EnemyHealthBar` (`WidgetComponent.GetUserWidgetObject` (`self.Widget`))))
  (`/Game/UI/WBP_EnemyHealthBar.SetHealth` _aswbp_enemy_health_bar (/ (`self.Health`) (`self.MaxHealth`))))

(fn `UserConstructionScript`)