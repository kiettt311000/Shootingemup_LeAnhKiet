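; BP_EnemyonPath is an actor, named as an enemy, that moves along its own spline path.
; On BeginPlay it detaches the spline keeping world transform, so the path stays put while the actor moves.
; A timeline, with play rate set from TravelTime, samples the spline at constant velocity and sets the actor's location with sweep on each update.
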(event `self.ReceiveBeginPlay`
  (`parent.ReceiveBeginPlay`)
  (`SceneComponent.K2_DetachFromComponent` (`self.Spline`) "KeepWorld" "KeepWorld" "KeepWorld" true)
  (`TimelineComponent.SetPlayRate` (`self.TL_Movealongspline`) (/ 1.0 (`self.TravelTime`)))
  (bind (_direction _time) (`Timeline|TL_Movealongspline`)
    (:`Update`
      (`self.K2_SetActorLocation` (`SplineComponent.GetLocationAtTime` (`self.Spline`) _time "World" true) true))))

(fn `UserConstructionScript`
  (`parent.UserConstructionScript`))