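; Enemy wave spawner that runs the sequence of waves defined in a data asset, starting on BeginPlay.
; After each wave's initial delay, it spawns members one by one with per-enemy delay, class and transform, messaging each its pickup-drop settings.
; It then polls the spawned list, pruning invalid actors, and advances once empty.
; After the last wave, it tells the HUD to show the end screen.
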(event `ContinueNext Wave`
  (bind _result (`/Engine/EditorBlueprintResources/StandardMacros.IncrementInt` (`self.CurrentWaveIndex`))
    (:`  `
      (bind _setofwave (`/Game/Framework/PDA_SetofWave.SetofWave` (stale `self.ReceiveBeginPlay` _wavedateasset)))
      (if (`KismetArrayLibrary.Array_IsValidIndex` _setofwave _result)
        (bind (_output_enemymembers _output_innitialwavedelay) (break `/Game/Framework/S_Wave` (`|GetArrayItem` _setofwave (`self.CurrentWaveIndex`))))
        (`KismetSystemLibrary.K2_SetTimerDelegate` (delegate `StartWave`) _output_innitialwavedelay :!label _label)
        (else
          (message `/Game/Framework/BPI_MyFlyingShmup.ShowEndScreen` (`PlayerController.GetHUD` (`GameplayStatics.GetPlayerController` 0)) true))))))

(event `self.ReceiveBeginPlay`
  (bind _wavedateasset (`self.WavedateAsset`)
    (:`then`
      (goto _label))
    (:`else`)))

(event `StartWave`
  (bind _output_enemymembers (break `/Game/Framework/S_Wave` (`|GetArrayItem` (`/Game/Framework/PDA_SetofWave.SetofWave` (`self.WavedateAsset`)) (`self.CurrentWaveIndex`))))
  (bind (_output_waveid _output_initialspawndelay _output_enemyclass _output_spawntransform _output_shoulddroppickup _output_pickupclass) (break `/Game/Framework/S_WaveEnemyMembers` (`|GetArrayItem` _output_enemymembers (`self.EnemyMembersIndex`))))
  (bind _output_get (set `self.EnemyMembersIndex` 0))
  (if (> _output_get (`KismetArrayLibrary.Array_LastIndex` _output_enemymembers)) :!label _label_2
    ; Remove any valid enemies
    (for (_array_element _array_index) (`self.SpawnedEnemies`) :!label _label_3
      (`/Engine/EditorBlueprintResources/StandardMacros.IsValid` _array_element
        (:`Is Not Valid`
          (`KismetArrayLibrary.Array_Remove` (`self.SpawnedEnemies`) _array_index))))
    ; Check if it empty
    (if (`KismetArrayLibrary.Array_IsEmpty` (`self.SpawnedEnemies`))
      (`self.ContinueNext Wave`)
      (else
        (`KismetSystemLibrary.Delay` 0.2)
        (goto _label_3)))
    (else
      (`KismetSystemLibrary.Delay` _output_initialspawndelay)
      (bind _returnvalue (`|SpawnActorFromClass` _output_enemyclass _output_spawntransform "AlwaysSpawn" "MultiplyWithRoot" null null))
      (message `/Game/Framework/BPI_MyFlyingShmup.AssignSpawnEnemyProp` _returnvalue _output_shoulddroppickup _output_pickupclass)
      (`KismetArrayLibrary.Array_Add` (`self.SpawnedEnemies`) _returnvalue)
      (`/Engine/EditorBlueprintResources/StandardMacros.IncrementInt` (`self.EnemyMembersIndex`)
        (:`  `
          (goto _label_2))))))

(fn `UserConstructionScript`)