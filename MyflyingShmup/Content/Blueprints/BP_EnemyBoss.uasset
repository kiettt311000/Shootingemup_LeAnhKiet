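; BP_EnemyBoss is an enemy boss that moves itself into the play area on spawn, then moves from side to side.
; BeginPlay calls the parent, then a timeline offsets the boss along Y from its start location.
; When that finishes, the boss re-caches its location and a second, slowed timeline drives it along X.
; Both moves use swept SetActorLocation calls scaled from timeline values.
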(event `self.ReceiveBeginPlay`
  (`parent.ReceiveBeginPlay`)
  (`self.EnterPlayArea`))

(event `EnterPlayArea`
  (set `self.InitialLocation` (`self.K2_GetActorLocation`))
  (bind (_direction _x_offset) (`Timeline|TL_EnterPlayArea` :!via `PlayFromStart`)
    (:`Update`
      (`self.K2_SetActorLocation` (+ (`self.InitialLocation`) (`KismetMathLibrary.MakeVector` 0.0 (* _x_offset -1600.0))) true))
    (:`Finished`
      (`self.Movesidetoside`))))

(event `Movesidetoside`
  (set `self.InitialLocation` (`self.K2_GetActorLocation`))
  (`TimelineComponent.SetPlayRate` (`self.TL_MoveSidetoSide`) 0.05)
  (bind (_direction _x_value) (`Timeline|TL_MoveSidetoSide` :!via `PlayFromStart`)
    (:`Update`
      (`self.K2_SetActorLocation` (+ (`self.InitialLocation`) (`KismetMathLibrary.MakeVector` (* _x_value 2000.0))) true))))

(fn `UserConstructionScript`
  (`parent.UserConstructionScript`))