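; Enemy spawner actor that keeps spawning random enemies from a class pool on a self-requeuing timer with a random delay.
; Each enemy appears at a random point on a start spline, rotated to face a random point on an end spline.
; It then receives a message with a small weighted chance to drop a random pickup on death.
; All randomness draws from one fixed-seed stream, set on BeginPlay.
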(event `self.ReceiveBeginPlay`
  (`KismetMathLibrary.SetRandomStreamSeed` (`self.RandomStream`) 102348)
  (`self.QueueEnemySpawn`))

(event `QueueEnemySpawn`
  (bind _returnvalue (`KismetSystemLibrary.K2_SetTimerDelegate` (delegate `Enemy`) (`KismetMathLibrary.RandomFloatInRangeFromStream` (`self.RandomStream`) 1.0 3.0) false true))
  (set `self.EnemySpawnTimer` _returnvalue))

(event `Enemy`
  (bind (_startloc _endloc) (`self.GetStartendEndLOC`))
  (bind _returnvalue (`|SpawnActorFromClass` (`KismetArrayLibrary.Array_RandomFromStream` (`self.EnemyClassPool`) (`self.RandomStream`)) (`KismetMathLibrary.MakeTransform` _startloc (`KismetMathLibrary.FindLookAtRotation` _startloc _endloc)) "Undefined" "MultiplyWithRoot" null null))
  (message `/Game/Framework/BPI_MyFlyingShmup.AssignSpawnEnemyProp` _returnvalue (`KismetMathLibrary.RandomBoolWithWeightFromStream` (`self.RandomStream`) 0.1) (`KismetArrayLibrary.Array_RandomFromStream` (`self.PickupClassPool`) (`self.RandomStream`)))
  (`self.QueueEnemySpawn`))

(fn `GetStartendEndLOC`
  (returns (StartLOC :type "Vector Structure") (EndLOC :type "Vector Structure"))
  (bind _returnvalue (`KismetMathLibrary.RandomFloatFromStream` (`self.RandomStream`)))
  (return (`SplineComponent.GetLocationAtTime` (`self.StartLOC`) _returnvalue "World" false) (`SplineComponent.GetLocationAtTime` (`self.EndLOC`) _returnvalue "World" false)))

(fn `UserConstructionScript`)