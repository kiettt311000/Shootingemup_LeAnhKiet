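; Player pawn that moves along fixed world axes using Enhanced Input and a FloatingPawnMovement component.
; On BeginPlay it adds its input mapping context to the local player subsystem, provided its controller is a PlayerController.
; Four separate input actions each feed a constant world-space vector on X or Y into the movement component, independent of pawn or camera rotation and input value.
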(event `self.ReceiveBeginPlay`
  ; add mapping context
  (bind _asplayer_controller (cast `PlayerController` (`self.GetController`)))
  (`EnhancedInputSubsystemInterface.AddMappingContext` (pcsubsystem `EnhancedInputLocalPlayerSubsystem` _asplayer_controller) "/Game/Input/IMC_Myfirstplayerpawn.IMC_Myfirstplayerpawn" 0 (struct)))

(event `EnhancedInput|/Game/Input/IA_MoveForward`
  (params (ActionValue :type Boolean) (ElapsedSeconds :type "Float (double-precision)") (TriggeredSeconds :type "Float (double-precision)") (InputAction :type "InputAction Object Reference" :default "/Game/Input/IA_MoveForward.IA_MoveForward"))
  ; PIA into Movement
  (:`Triggered`
    (`PawnMovementComponent.AddInputVector` (`self.FloatingPawnMovement`) (1.0 0.0 0.0) false)))

(event `EnhancedInput|/Game/Input/IA_MoveBackward`
  (params (ActionValue :type Boolean) (ElapsedSeconds :type "Float (double-precision)") (TriggeredSeconds :type "Float (double-precision)") (InputAction :type "InputAction Object Reference" :default "/Game/Input/IA_MoveBackward.IA_MoveBackward"))
  ; PIA into Movement
  (:`Triggered`
    (`PawnMovementComponent.AddInputVector` (`self.FloatingPawnMovement`) (-1.0 0.0 0.0) false)))

(event `EnhancedInput|/Game/Input/IA_MoveLeft`
  (params (ActionValue :type Boolean) (ElapsedSeconds :type "Float (double-precision)") (TriggeredSeconds :type "Float (double-precision)") (InputAction :type "InputAction Object Reference" :default "/Game/Input/IA_MoveLeft.IA_MoveLeft"))
  ; PIA into Movement
  (:`Triggered`
    (`PawnMovementComponent.AddInputVector` (`self.FloatingPawnMovement`) (0.0 -1.0 0.0) false)))

(event `EnhancedInput|/Game/Input/IA_Moveright`
  (params (ActionValue :type Boolean) (ElapsedSeconds :type "Float (double-precision)") (TriggeredSeconds :type "Float (double-precision)") (InputAction :type "InputAction Object Reference" :default "/Game/Input/IA_Moveright.IA_Moveright"))
  ; PIA into Movement
  (:`Triggered`
    (`PawnMovementComponent.AddInputVector` (`self.FloatingPawnMovement`) (0.0 1.0 0.0) false)))

(fn `UserConstructionScript`)